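; Player controller for the Bomberman game that toggles the pause menu from the IA_Pause input action.
; The validity of the stored PauseMenuRef serves as the toggle state.
; Pausing creates WBP_PauseMenu, adds it to the viewport and shows the mouse cursor.
; Unpausing removes and clears the widget, hides the cursor and restores game-only input, with a debug print.
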(event Input|EnhancedActionEvents|EnhancedInputActionIA_Pause
  (params (ActionValue :type Boolean) (ElapsedSeconds :type Float%20%28double-precision%29) (TriggeredSeconds :type Float%20%28double-precision%29) (InputAction :type Input%20Action%20Object%20Reference :default "/Game/Input/Actions/IA_Pause.IA_Pause"))
  (bind _returnvalue (Game|GetPlayerController 0))
  (:Started
    (Utilities|IsValid (Variables|Default|GetPauseMenuRef)
      (:Is%20Valid
        (Development|PrintString "Is Valid")
        (Game|SetGamePaused false)
        (Widget|RemovefromParent (Variables|Default|GetPauseMenuRef))
        (Variables|/Script/Engine.PlayerController|SetbShowMouseCursor _returnvalue false)
        (Input|SetInputModeGameOnly _returnvalue false)
        (Variables|Default|SetPauseMenuRef 0))
      (:Is%20Not%20Valid
        (Game|SetGamePaused true)
        (bind _returnvalue_2 (UserInterface|CreateWidget "/Game/Blueprints/UI/WBP_PauseMenu.WBP_PauseMenu_C"))
        (bind _output_get (Variables|Default|SetPauseMenuRef _returnvalue_2))
        (UserInterface|Viewport|AddtoViewport _output_get 0)
        (Variables|/Script/Engine.PlayerController|SetbShowMouseCursor (Game|GetPlayerController 0) true)))))

(fn ConstructionScript)