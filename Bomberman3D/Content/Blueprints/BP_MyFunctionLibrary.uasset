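; Blueprint function library of shared helpers for a Bomberman game: cast-failure reporting and match info text.
; GetAndFormatMatchInfo reads score and lives from the first BombermanPlayerState, plus stage and time remaining from BombermanGameState, and returns them as labeled text.
; A Sequence runs both casts before formatting; a failed cast calls CastFailed, which prints an error naming the type, and returns fallback "Something Went Wrong" values.
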(fn CastFailed
  (params (CastToWhatFailed :type String))
  (bind _returnvalue (Utilities|Text|ToText(String) CastToWhatFailed))
  (bind _result (Utilities|Text|FormatText "Cast to {Object} failed!" _returnvalue))
  (bind _returnvalue_2 (Utilities|String|ToString(Text) _result))
  (Development|PrintString 0 _returnvalue_2)
  (return _returnvalue_2))

(fn GetandFormatMatchInfo
  (Utilities|FlowControl|Sequence
    (:then_0
      (bind _asbomberman_player_state (Utilities|Casting|CastToBombermanPlayerState (Game|GetPlayerState 0))
        (:CastFailed
          ;[0.15 0.15 0.15 0.5] If fails (it wont, but just in case)
          (CallFunction|CastFailed "BombermanPlayerState"))))
    (:then_1
      (bind _asbomberman_game_state (Utilities|Casting|CastToBombermanGameState (Game|GetGameState))
        (:CastFailed
          (CallFunction|CastFailed "BombermanGameState"))))
    (:then_2
      (return (Utilities|Text|FormatText "Score: {0}" (Variables|/Script/Engine.PlayerState|GetScore _asbomberman_player_state)) (Utilities|Text|FormatText "Lives: {0}" (Variables|/Script/Bomberman3D.BombermanPlayerState|GetLives _asbomberman_player_state)) (Utilities|Text|FormatText "Time remaining: {0}" (Variables|/Script/Bomberman3D.BombermanGameState|GetStageTimeRemaining _asbomberman_game_state)) (Utilities|Text|FormatText "Stage: {0}" (Variables|/Script/Bomberman3D.BombermanGameState|GetCurrentStage _asbomberman_game_state)))))
  (return "Something Went Wrong" "Something Went Wrong" "Something Went Wrong" "Something Went Wrong"))